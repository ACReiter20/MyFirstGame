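; BP_Fire2 is a fire hazard that deals periodic damage to the first-person character while it is inside the Box trigger.
; Box begin overlap stores the character and starts a looping timer that applies fixed damage every two seconds, with no immediate hit on entry.
; Box end overlap by that character type clears the timer through its stored handle, stopping the damage.
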(event OnComponentBeginOverlap(Box)
  (params (OverlappedComponent :type Primitive%20Component%20Object%20Reference) (OtherActor :type Actor%20Object%20Reference) (OtherComp :type Primitive%20Component%20Object%20Reference) (OtherBodyIndex :type Integer) (bFromSweep :type Boolean) (SweepResult :type Hit%20Result%20Structure%20%28by%20ref%29))
  (bind _asbp_first_person_character (Utilities|Casting|CastToBP_FirstPersonCharacter OtherActor))
  (Variables|Default|SetAs%20BP%20First%20Person%20Character _asbp_first_person_character)
  (bind _returnvalue (Utilities|Time|SetTimerbyEvent (delegate Custom|DamagePlayer) 2.0 true))
  (Variables|Default|SetTimerRef _returnvalue))

(event OnComponentEndOverlap(Box)
  (params (OverlappedComponent :type Primitive%20Component%20Object%20Reference) (OtherActor :type Actor%20Object%20Reference) (OtherComp :type Primitive%20Component%20Object%20Reference) (OtherBodyIndex :type Integer))
  (Utilities|Casting|CastToBP_FirstPersonCharacter OtherActor)
  (Utilities|Time|ClearandInvalidateTimerbyHandle (Variables|Default|GetTimerRef)))

(event Custom|DamagePlayer
  (Game|Damage|ApplyDamage (Variables|Default|GetAs%20BP%20First%20Person%20Character) 2e+01 0 0))

(fn ConstructionScript)