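; BP_Ladder is a ladder actor that drops into place and lets the first-person player climb it.
; Tick polls the character's Ladder flag and, while it is set, uses MoveComponentTo to slide and rotate the ladder to a fixed relative pose.
; Box overlaps toggle the actor's input, so pressing E inside moves the player's capsule straight up over time, rotated to match the ladder.
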(event OnComponentBeginOverlap(Box)
  (params (OverlappedComponent :type Primitive%20Component%20Object%20Reference) (OtherActor :type Actor%20Object%20Reference) (OtherComp :type Primitive%20Component%20Object%20Reference) (OtherBodyIndex :type Integer) (bFromSweep :type Boolean) (SweepResult :type Hit%20Result%20Structure%20%28by%20ref%29))
  (Utilities|Casting|CastToBP_FirstPersonCharacter OtherActor)
  (Input|EnableInput (Game|GetPlayerController 0)))

(event OnComponentEndOverlap(Box)
  (params (OverlappedComponent :type Primitive%20Component%20Object%20Reference) (OtherActor :type Actor%20Object%20Reference) (OtherComp :type Primitive%20Component%20Object%20Reference) (OtherBodyIndex :type Integer))
  (Utilities|Casting|CastToBP_FirstPersonCharacter OtherActor)
  (Input|DisableInput (Game|GetPlayerController 0)))

(event EventTick
  (params (DeltaSeconds :type Float%20%28single-precision%29))
  (bind _asbp_first_person_character (Utilities|Casting|CastToBP_FirstPersonCharacter (Game|GetPlayerCharacter 0)))
  (if (Variables|/Game/FirstPerson/Blueprints/BP_FirstPersonCharacter.BP_FirstPersonCharacter_C|GetLadder _asbp_first_person_character)
    (Components|MoveComponentTo (Variables|Default|GetLadder) "0.000000,0.000000,-390.000000" "0.000000,-90.000000,0.000000" false false 1.0 false)))

(event Input|KeyboardEvents|E
  (params (Key :type Key%20Structure :default "None"))
  (:Pressed
    (bind _asbp_first_person_character (Utilities|Casting|CastToBP_FirstPersonCharacter (Game|GetPlayerCharacter 0)))
    (Components|MoveComponentTo (Variables|/Script/Engine.Character|GetCapsuleComponent _asbp_first_person_character) (+ (Transformation|GetWorldLocation (Variables|/Script/Engine.Character|GetCapsuleComponent _asbp_first_person_character)) "0.000000,0.000000,500.000000") (Transformation|GetWorldRotation (Variables|Default|GetLadder)) false false 2.0 false)))

(fn ConstructionScript)