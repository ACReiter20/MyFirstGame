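; Searchable chest, optionally pin-locked, that grants the first-person character a key once.
; Box overlap with the player enables input; end overlap also calls EnableInput, so input is never disabled.
; While locked, E toggles a keypad widget and cursor, and AddToPin unlocks and closes it when the entry matches Pin.
; Once unlocked, E sets HasFiKey on the character and prints a message.
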(event OnComponentBeginOverlap(Box)
  (params (OverlappedComponent :type Primitive%20Component%20Object%20Reference) (OtherActor :type Actor%20Object%20Reference) (OtherComp :type Primitive%20Component%20Object%20Reference) (OtherBodyIndex :type Integer) (bFromSweep :type Boolean) (SweepResult :type Hit%20Result%20Structure%20%28by%20ref%29))
  (Utilities|Casting|CastToBP_FirstPersonCharacter OtherActor)
  (Input|EnableInput (Game|GetPlayerController 0)))

(event OnComponentEndOverlap(Box)
  (params (OverlappedComponent :type Primitive%20Component%20Object%20Reference) (OtherActor :type Actor%20Object%20Reference) (OtherComp :type Primitive%20Component%20Object%20Reference) (OtherBodyIndex :type Integer))
  (Utilities|Casting|CastToBP_FirstPersonCharacter OtherActor)
  (Input|EnableInput (Game|GetPlayerController 0)))

(event Input|KeyboardEvents|E
  (params (Key :type Key%20Structure :default "None"))
  (bind _returnvalue (Game|GetPlayerController 0))
  (:Pressed
    (if (Variables|Default|GetLocked)
      (Utilities|IsValid (Variables|Default|GetPinWigRef)
        (:Is%20Valid
          (Widget|RemovefromParent (stale _output_get))
          (Variables|Default|SetPinWigRef 0)
          (Input|SetInputModeGameOnly _returnvalue false)
          (Variables|/Script/Engine.PlayerController|SetbShowMouseCursor _returnvalue false))
        (:Is%20Not%20Valid
          (bind _returnvalue_2 (UserInterface|CreateWidget "/Game/Blueprints/Box/BPWIG_KeyPad.BPWIG_KeyPad_C" 0 self))
          (bind _output_get (Variables|Default|SetPinWigRef _returnvalue_2))
          (UserInterface|Viewport|AddtoViewport _output_get 0)
          (Input|SetInputModeGameandUI _returnvalue (Variables|Default|GetPinWigRef) "DoNotLock" false false)
          (Variables|/Script/Engine.PlayerController|SetbShowMouseCursor _returnvalue true)))
      (elif (not (Variables|Default|GetHasSearched))
        (Variables|Default|SetHasSearched true)
        (bind _asbp_first_person_character (Utilities|Casting|CastToBP_FirstPersonCharacter (stale OnComponentBeginOverlap(Box) OtherActor)))
        (Variables|/Game/FirstPerson/Blueprints/BP_FirstPersonCharacter.BP_FirstPersonCharacter_C|SetHasFiKey _asbp_first_person_character true)
        (Development|PrintString "You got a key")))))

(fn ConstructionScript)

(fn AddtoPin
  (params (Input :type Integer))
  (bind _returnvalue (Game|GetPlayerController 0))
  (if (== Input (Variables|Default|GetPin))
    (Variables|Default|SetLocked false)
    (Widget|RemovefromParent (Variables|Default|GetPinWigRef))
    (Input|SetInputModeGameOnly _returnvalue false)
    (Variables|/Script/Engine.PlayerController|SetbShowMouseCursor _returnvalue false)))